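; Door manager that spawns doors around the rooms neighbouring the player and registers itself on the Siim game instance.
; On begin play and whenever the room manager generates coordinates, it waits briefly, then finds the room centre closest to the player.
; It offsets that centre by the grid step along ±X, ±Y and ±Z, spawns BP_Door at each angle per location without duplicate checks, then broadcasts DoorsGenerated.
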(event `self.ReceiveBeginPlay`
  (bind _asgame_instance_siim (cast `/Game/Siim/GameInstanceSiim` (`GameplayStatics.GetGameInstance`)))
  (set `/Game/Siim/GameInstanceSiim.DoorManager` self _asgame_instance_siim)
  (add `/Game/Siim/BP_RoomManager.CoordinatesGenerated` (`self.BP_RoomManager`) (delegate `GenerateNeighbouringDoors`))
  (`self.GenerateNeighbouringDoors`))

(event `GenerateNeighbouringDoors`
  (bind _neighbouringcubelocations (`self.NeighbouringCubeLocations`))
  (`KismetSystemLibrary.Delay` 0.2)
  ;[1 1 1] Get nearest centerpoint from the player
  (bind _asbp_third_person_character_siim (cast `/Game/Siim/BP_ThirdPersonCharacter_Siim` (`GameplayStatics.GetPlayerCharacter` 0)))
  (bind _roommanager (`/Game/Siim/GameInstanceSiim.RoomManager` (stale `self.ReceiveBeginPlay` _asgame_instance_siim)))
  (bind _closest (`/Game/Siim/FunctionLibraryGeoMob.FindClosestVector` (`/Game/Siim/BP_RoomManager.AllCubeLocations` _roommanager) (`SceneComponent.K2_GetComponentLocation` (`Character.CapsuleComponent` _asbp_third_person_character_siim))))
  (`|ExecutionSequence`
    (:`then_0`
      (bind _x (.x _closest))
      (bind _y (.y _closest))
      (bind _z (.z _closest))
      (bind (_stepxyz_x _stepxyz_y _stepxyz_z) (`KismetMathLibrary.BreakVector` (`/Game/Siim/BP_RoomManager.StepXYZ` _roommanager)))
      (`KismetArrayLibrary.Array_Add` _neighbouringcubelocations (`KismetMathLibrary.MakeVector` (- _x _stepxyz_x) _y _z)))
    (:`then_1`
      (`KismetArrayLibrary.Array_Add` _neighbouringcubelocations (`KismetMathLibrary.MakeVector` (+ _x _stepxyz_x) _y _z)))
    (:`then_2`
      (bind _x_2 (.x _closest))
      (bind _y_2 (.y _closest))
      (bind _z_2 (.z _closest))
      (`KismetArrayLibrary.Array_Add` _neighbouringcubelocations (`KismetMathLibrary.MakeVector` _x_2 (- _y_2 _stepxyz_y) _z_2)))
    (:`then_3`
      (`KismetArrayLibrary.Array_Add` _neighbouringcubelocations (`KismetMathLibrary.MakeVector` _x_2 (+ _y_2 _stepxyz_y) _z_2)))
    (:`then_4`
      (bind _x_3 (.x _closest))
      (bind _y_3 (.y _closest))
      (bind _z_3 (.z _closest))
      (`KismetArrayLibrary.Array_Add` _neighbouringcubelocations (`KismetMathLibrary.MakeVector` _x_3 _y_3 (- _z_3 _stepxyz_z))))
    (:`then_5`
      (`KismetArrayLibrary.Array_Add` _neighbouringcubelocations (`KismetMathLibrary.MakeVector` _x_3 _y_3 (+ _z_3 _stepxyz_z))))
    (:`then_6`
      (bind _asgame_instance_siim (cast `/Game/Siim/GameInstanceSiim` (`GameplayStatics.GetGameInstance`)))
      (set `/Game/Siim/GameInstanceSiim.NeigbouringRoomLocations` _neighbouringcubelocations _asgame_instance_siim))
    (:`then_7`
      ;[1 1 1] Create 4 Doors to all 6 location (also need to check if door already exists)
      (for _array_element (`self.NeighbouringCubeLocations`)
        (for _array_element_2 (`self.DoorAngles`)
          (`|SpawnActorFromClass` "/Game/Siim/BP_Door.BP_Door_C" (`KismetMathLibrary.MakeTransform` _array_element (`KismetMathLibrary.MakeRotator` 0.0 0.0 _array_element_2)) "Undefined" "OverrideRootScale" null null))))
    (:`then_9`
      (`self.DoorsGenerated`))))

(fn `UserConstructionScript`)