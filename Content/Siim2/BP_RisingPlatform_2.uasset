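; Elevator platform actor that offers an up/down choice through a UI_UpDown widget when BP_ThirdPersonCharacter_Siim enters its Box trigger.
; Entering shows the widget and disables input and movement; leaving Box1 restores them and resets the move's DoOnce.
; The widget's choice plays one of two timelines driving a swept location lerp.
; As wired, both lerp endpoints equal the current location, and the RoomManager step offsets in the construction script never run.
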(event `self.ReceiveBeginPlay`
  (bind _returnvalue (`|CreateWidget` "/Game/Siim/UI_Up-Down.UI_Up-Down_C" (`GameplayStatics.GetPlayerController` 0)))
  (bind _output_get (set `self.WidgetUpAndDown` _returnvalue))
  (`UserWidget.AddToViewport` _output_get 0)
  (`Widget.SetVisibility` _output_get "Hidden")
  (add `/Game/Siim/UI_Up-Down.UpOrDown` _output_get (delegate `GoesUpOrDown`)))

(event `GoesUpOrDown`
  (params (IsUp :type Boolean))
  (bind _currentlocation (`self.CurrentLocation`))
  (bind _x (.x _currentlocation))
  (bind _y (.y _currentlocation))
  (bind _z (.z _currentlocation))
  ;[1 1 1] UP-DOWN movement
  (cast `/Game/Siim/GameInstanceSiim` (`GameplayStatics.GetGameInstance`))
  (set `self.CurrentLocation` (`self.K2_GetActorLocation`))
  (`/Engine/EditorBlueprintResources/StandardMacros.DoOnce` false :!label _label
    (:`Completed`
      (if IsUp
        (bind (_direction _newtrack_0) (`Timeline|Timeline_0` :!via `PlayFromStart`)
          (:`Update`
            (bind _returnvalue (`KismetMathLibrary.VLerp` _currentlocation (`KismetMathLibrary.MakeVector` _x _y _z) _newtrack_0))
            (`self.K2_SetActorLocation` _returnvalue true))
          (:`Finished`
            (set `self.CurrentLocation` _returnvalue)))
        (else
          (bind (_direction_2 _newtrack_0_2) (`Timeline|Timeline_1` :!via `PlayFromStart`)
            (:`Update`
              (bind _returnvalue_2 (`KismetMathLibrary.VLerp` _currentlocation (`KismetMathLibrary.MakeVector` _x _y _z) _newtrack_0_2))
              (`self.K2_SetActorLocation` _returnvalue_2 true))
            (:`Finished`
              (set `self.CurrentLocation` _returnvalue_2))))))))

(event `self.Box.OnComponentEndOverlap`
  (params (OverlappedComponent :type "PrimitiveComponent Object Reference") (OtherActor :type "Actor Object Reference") (OtherComp :type "PrimitiveComponent Object Reference") (OtherBodyIndex :type Integer)))

(event `self.Box1.OnComponentEndOverlap`
  (params (OverlappedComponent :type "PrimitiveComponent Object Reference") (OtherActor :type "Actor Object Reference") (OtherComp :type "PrimitiveComponent Object Reference") (OtherBodyIndex :type Integer))
  ;[1 1 1] UP-DOWN movement
  (`/Game/Siim/FunctionLibraryGeoMob.EnableInputAndMovement`)
  (goto _label :!via `Reset`))

(event `self.Box.OnComponentBeginOverlap`
  (params (OverlappedComponent :type "PrimitiveComponent Object Reference") (OtherActor :type "Actor Object Reference") (OtherComp :type "PrimitiveComponent Object Reference") (OtherBodyIndex :type Integer) (bFromSweep :type Boolean) (SweepResult :type "HitResult Structure (by ref)"))
  ;[1 1 1] Open Up-Down menu, disable outputs etc
  (cast `/Game/Siim/BP_ThirdPersonCharacter_Siim` OtherActor)
  (`Widget.SetVisibility` (`self.WidgetUpAndDown`) "Visible")
  (`/Game/Siim/FunctionLibraryGeoMob.DisableInputAndMovement`))

(fn `UserConstructionScript`)