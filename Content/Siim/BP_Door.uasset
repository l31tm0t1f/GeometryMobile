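; BP_Door is a sliding door that rises when BP_ThirdPersonCharacter_Siim enters its trigger box and lowers when that character leaves.
; BeginPlay stores the door's starting relative location and derives the travel distance from the mesh's bounding box height.
; A timeline lerps the door upward by that height, playing from the start on entry and reversing from the end on exit, when it also calls DoorCloses.
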(event `self.ReceiveBeginPlay`
  (bind _returnvalue (`StaticMesh.GetBoundingBox` (`StaticMeshComponent.StaticMesh` (`self.Door`))))
  ;[1 1 1] Get/Set Door height (distance how much door moves)
  (set `self.Height_Door` (- (.z (`.Max` (break `Box` _returnvalue))) (.z (break `Box` _returnvalue))))
  (set `self.RelLoc_Door` (`SceneComponent.RelativeLocation` (`self.Door`))))

(event `self.Box.OnComponentBeginOverlap`
  (params (OverlappedComponent :type "PrimitiveComponent Object Reference") (OtherActor :type "Actor Object Reference") (OtherComp :type "PrimitiveComponent Object Reference") (OtherBodyIndex :type Integer) (bFromSweep :type Boolean) (SweepResult :type "HitResult Structure (by ref)"))
  (bind _relloc_door (`self.RelLoc_Door`))
  (cast `/Game/Siim/BP_ThirdPersonCharacter_Siim` OtherActor)
  ;[1 1 1] Moving the door
  (bind (_direction _newtrack_0) (`Timeline|Timeline_0` :!via `PlayFromStart` :!label _label)
    (:`Update`
      (`SceneComponent.K2_SetRelativeLocation` (`self.Door`) (`KismetMathLibrary.VLerp` _relloc_door (`KismetMathLibrary.MakeVector` (.x _relloc_door) (.y _relloc_door) (+ (.z _relloc_door) (`self.Height_Door`))) _newtrack_0) false false))))

(event `self.Box.OnComponentEndOverlap`
  (params (OverlappedComponent :type "PrimitiveComponent Object Reference") (OtherActor :type "Actor Object Reference") (OtherComp :type "PrimitiveComponent Object Reference") (OtherBodyIndex :type Integer))
  (cast `/Game/Siim/BP_ThirdPersonCharacter_Siim` OtherActor)
  ;[1 1 1] Call Door Closes
  (`self.DoorCloses`)
  (goto _label :!via `ReverseFromEnd`))

(fn `UserConstructionScript`)