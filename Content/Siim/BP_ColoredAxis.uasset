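; BP_ColoredAxis is an actor that draws labeled X, Y and Z axis markers at every cube location in the room.
; After a short BeginPlay delay, it gets the RoomManager from GameInstanceSiim, builds the axes and binds the same build to CoordinatesGenerated.
; Each location gets runtime-added static mesh components for three axes and their offset 3D text labels.
; Rebuilds add components without clearing earlier ones.
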(event `CreateAllAxes`
  (for _array_element (`/Game/Siim/BP_RoomManager.AllCubeLocations` (`self.RoomManager`))
    (`|ExecutionSequence`
      (:`then_0`
        (bind _returnvalue (`AddComponent|NODE_AddStaticMeshComponent-0` :`RelativeTransform` (`KismetMathLibrary.MakeTransform` _array_element (struct :`Yaw` 90.0))))
        (`StaticMeshComponent.SetStaticMesh` _returnvalue "/Game/Siim/SM/X_.X_")
        (bind _returnvalue_2 (`AddComponent|NODE_AddStaticMeshComponent-4` :`RelativeTransform` (`KismetMathLibrary.MakeTransform` (- _array_element (400.0 110.0 -25.0)) (struct :`Yaw` -90.0 :`Roll` 90.0) (0.03 0.03 0.03))))
        (`StaticMeshComponent.SetStaticMesh` _returnvalue_2 "/Game/Siim/SM/3DText_X.3DText_X"))
      (:`then_1`
        (bind _returnvalue_3 (`AddComponent|NODE_AddStaticMeshComponent-3` :`RelativeTransform` (`KismetMathLibrary.MakeTransform` _array_element)))
        (`StaticMeshComponent.SetStaticMesh` _returnvalue_3 "/Game/Siim/SM/Y.Y")
        (bind _returnvalue_4 (`AddComponent|NODE_AddStaticMeshComponent-5` :`RelativeTransform` (`KismetMathLibrary.MakeTransform` (- _array_element (130.0 400.0 -25.0)) (struct :`Roll` 90.0) (0.03 0.03 0.03))))
        (`StaticMeshComponent.SetStaticMesh` _returnvalue_4 "/Game/Siim/SM/3DText_Y.3DText_Y"))
      (:`then_2`
        (bind _returnvalue_5 (`AddComponent|NODE_AddStaticMeshComponent-2` :`RelativeTransform` (`KismetMathLibrary.MakeTransform` _array_element (struct :`Yaw` 90.0))))
        (`StaticMeshComponent.SetStaticMesh` _returnvalue_5 "/Game/Siim/SM/Z.Z")
        (bind _returnvalue_6 (`AddComponent|NODE_AddStaticMeshComponent-6` :`RelativeTransform` (`KismetMathLibrary.MakeTransform` (- _array_element (400.0 390.0 -320.0)) (struct :`Yaw` -45.0 :`Roll` 90.0) (0.03 0.03 0.03))))
        (`StaticMeshComponent.SetStaticMesh` _returnvalue_6 "/Game/Siim/SM/3DText_Z.3DText_Z")))))

(event `self.ReceiveBeginPlay`
  (`KismetSystemLibrary.Delay` 0.2)
  (bind _asgame_instance_siim (cast `/Game/Siim/GameInstanceSiim` (`GameplayStatics.GetGameInstance`)))
  (bind _output_get (set `self.RoomManager` (`/Game/Siim/GameInstanceSiim.RoomManager` _asgame_instance_siim)))
  (add `/Game/Siim/BP_RoomManager.CoordinatesGenerated` _output_get (delegate `CreateAllAxes`))
  (`self.CreateAllAxes`))

(fn `UserConstructionScript`)