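; BP_TaskUI is a Blueprint meant to build a 3D cube formation for a map from room coordinates.
; On BeginPlay, after a short delay, it gets the RoomManager from GameInstanceSiim, binds Create3DforMap to its coordinates-generated event, and calls it immediately.
; Create3DforMap is unfinished: it adds one static mesh component with no mesh assigned, and RoomManager's CorrectCubeLocations is left unused.
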(event `Create3DforMap`
  ;[1 1 1] CREATE Cube Formation according to placement
  (bind _returnvalue (`AddComponent|NODE_AddStaticMeshComponent-0`))
  (`StaticMeshComponent.SetStaticMesh` _returnvalue null))

(event `self.ReceiveBeginPlay`
  (`KismetSystemLibrary.Delay` 0.2)
  (bind _asgame_instance_siim (cast `/Game/Siim/GameInstanceSiim` (`GameplayStatics.GetGameInstance`)))
  (bind _output_get (set `self.RoomManager` (`/Game/Siim/GameInstanceSiim.RoomManager` _asgame_instance_siim)))
  (add `/Game/Siim/BP_RoomManager.CoordinatesGenerated` _output_get (delegate `Create3DforMap`))
  (`self.Create3DforMap`))

(fn `UserConstructionScript`)