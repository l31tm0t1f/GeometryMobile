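; BP_DoorManager spawns the doors between generated rooms, running after BeginPlay and binding to the RoomManager's CoordinatesGenerated event.
; Each run stores the six axis-aligned neighbours of the room centre nearest the player in the GameInstance.
; It then spawns a BP_Door per angle at every room location, not just neighbours.
; Duplicates are destroyed by comparing box positions against BPDoorArray, which is only appended inside that comparison loop.
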(event `self.ReceiveBeginPlay`
  (`KismetSystemLibrary.Delay` 0.2)
  (bind _asgame_instance_siim (cast `/Game/Siim/GameInstanceSiim` (`GameplayStatics.GetGameInstance`)))
  (bind _output_get (set `self.BP_RoomManager` (`/Game/Siim/GameInstanceSiim.RoomManager` _asgame_instance_siim)))
  (add `/Game/Siim/BP_RoomManager.CoordinatesGenerated` _output_get (delegate `GenerateNeighbouringDoors`))
  (`KismetSystemLibrary.Delay` 0.2)
  (`self.GenerateNeighbouringDoors`))

(event `GenerateNeighbouringDoors`
  (bind _neighbouringcubelocations (`self.NeighbouringCubeLocations`))
  (bind (_stepxyz_x _stepxyz_y _stepxyz_z) (`KismetMathLibrary.BreakVector` (`/Game/Siim/BP_RoomManager.StepXYZ` (`self.BP_RoomManager`))))
  ;[1 1 1] Get nearest centerpoint from the player
  (bind _asbp_third_person_character_siim (cast `/Game/Siim/BP_ThirdPersonCharacter_Siim` (`GameplayStatics.GetPlayerCharacter` 0)))
  (bind _allcubelocations (`/Game/Siim/BP_RoomManager.AllCubeLocations` (stale `self.ReceiveBeginPlay` _output_get)))
  (bind _closest (`/Game/Siim/FunctionLibraryGeoMob.FindClosestVector` _allcubelocations (`SceneComponent.K2_GetComponentLocation` (`Character.CapsuleComponent` _asbp_third_person_character_siim))))
  (`|ExecutionSequence`
    (:`then_0`
      (bind _x (.x _closest))
      (bind _y (.y _closest))
      (bind _z (.z _closest))
      (`KismetArrayLibrary.Array_Add` _neighbouringcubelocations (`KismetMathLibrary.MakeVector` (- _x _stepxyz_x) _y _z)))
    (:`then_1`
      (`KismetArrayLibrary.Array_Add` _neighbouringcubelocations (`KismetMathLibrary.MakeVector` (+ _x _stepxyz_x) _y _z)))
    (:`then_2`
      (bind _x_2 (.x _closest))
      (bind _y_2 (.y _closest))
      (bind _z_2 (.z _closest))
      (`KismetArrayLibrary.Array_Add` _neighbouringcubelocations (`KismetMathLibrary.MakeVector` _x_2 (- _y_2 _stepxyz_y) _z_2)))
    (:`then_3`
      (`KismetArrayLibrary.Array_Add` _neighbouringcubelocations (`KismetMathLibrary.MakeVector` _x_2 (+ _y_2 _stepxyz_y) _z_2)))
    (:`then_4`
      (bind _x_3 (.x _closest))
      (bind _y_3 (.y _closest))
      (bind _z_3 (.z _closest))
      (`KismetArrayLibrary.Array_Add` _neighbouringcubelocations (`KismetMathLibrary.MakeVector` _x_3 _y_3 (- _z_3 _stepxyz_z))))
    (:`then_5`
      (`KismetArrayLibrary.Array_Add` _neighbouringcubelocations (`KismetMathLibrary.MakeVector` _x_3 _y_3 (+ _z_3 _stepxyz_z))))
    (:`then_6`
      (bind _asgame_instance_siim (cast `/Game/Siim/GameInstanceSiim` (`GameplayStatics.GetGameInstance`)))
      (set `/Game/Siim/GameInstanceSiim.NeigbouringRoomLocations` _neighbouringcubelocations _asgame_instance_siim))
    (:`then_8`
      ;[1 1 1] Create ALL Doors (but avoid double doors)
      (for _array_element _allcubelocations
        (for _array_element_2 (`self.DoorAngles`)
          (bind _returnvalue (`|SpawnActorFromClass` "/Game/Siim/BP_Door.BP_Door_C" (`KismetMathLibrary.MakeTransform` _array_element (`KismetMathLibrary.MakeRotator` 0.0 0.0 _array_element_2)) "AlwaysSpawn" "OverrideRootScale" null null))
          (for _array_element_3 (`self.BP_DoorArray`)
            (if (== (`SceneComponent.K2_GetComponentLocation` (`/Game/Siim/BP_Door.Box` _array_element_3)) (`SceneComponent.K2_GetComponentLocation` (`/Game/Siim/BP_Door.Box` _returnvalue)) :`ErrorTolerance` 10.0)
              (`self.K2_DestroyActor` _returnvalue)
              (else
                (`KismetArrayLibrary.Array_Add` (`self.BP_DoorArray`) _returnvalue)))))))))

(fn `UserConstructionScript`)