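; BP_RoomManager procedurally builds a path of cube rooms surrounded by "death" cubes.
; The construction script lays three rows from the origin along shuffled random X/Y/Z directions, then fills unoccupied six-way neighbours with death cubes, recording all locations.
; CreateCube assembles rooms from floor, wall and ceiling mesh components, spaced by mesh bounds.
; BeginPlay registers the manager on GameInstanceSiim and calls CallCoordinatesGenerated; platform-placement logic is unconnected.
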(event `self.ReceiveBeginPlay`
  (bind _asgame_instance_siim (cast `/Game/Siim/GameInstanceSiim` (`GameplayStatics.GetGameInstance`)))
  (bind _output_get (set `/Game/Siim/GameInstanceSiim.RoomManager` self _asgame_instance_siim))
  (`self.CoordinatesGenerated` _output_get))

(fn `CreateCube`
  (params (VectorIn :type "Vector Structure"))
  (returns (VectorOut :type "Vector Structure"))
  (bind (_stepxyz_x _stepxyz_y _stepxyz_z) (`KismetMathLibrary.BreakVector` (`self.StepXYZ`)))
  (bind _returnvalue (`StaticMesh.GetBoundingBox` (`self.Floor`)))
  ;[1 1 1] Make 1 Cube
  (`|ExecutionSequence`
    (:`then_0`
      (bind _returnvalue_2 (`AddComponent|NODE_AddStaticMeshComponent-6` :`RelativeTransform` (`KismetMathLibrary.MakeTransform` VectorIn)))
      (`StaticMeshComponent.SetStaticMesh` _returnvalue_2 (`self.Floor`)))
    (:`then_1`
      (for _index (range 4)
        (bind _returnvalue_3 (`AddComponent|NODE_AddStaticMeshComponent-7` :`RelativeTransform` (`KismetMathLibrary.MakeTransform` VectorIn (`KismetMathLibrary.MakeRotator` 0.0 0.0 (`KismetMathLibrary.Conv_IntToDouble` (* _index 90))))))
        (`StaticMeshComponent.SetStaticMesh` _returnvalue_3 (`self.Wall`))))
    (:`then_2`
      (bind _returnvalue_4 (`AddComponent|NODE_AddStaticMeshComponent-11` :`RelativeTransform` (`KismetMathLibrary.MakeTransform` (+ VectorIn (`KismetMathLibrary.MakeVector` 0.0 0.0 (- _stepxyz_z (- (.z (`.Max` (break `Box` _returnvalue))) (.z (break `Box` _returnvalue)))))))))
      (`StaticMeshComponent.SetStaticMesh` _returnvalue_4 (`self.Floor`)))
    (:`then_3`)
    (:`then_5`
      (return VectorIn))))

(fn `UserConstructionScript`
  (bind (_stepxyz_x _stepxyz_y _stepxyz_z) (`KismetMathLibrary.BreakVector` (`self.StepXYZ`)))
  (bind _unitvectorarraynew (`self.UnitVectorArrayNEW`))
  (bind _arraystepcubesides (`self.ArrayStepCubeSides`))
  (bind (_currentposition_x _currentposition_y _currentposition_z) (`KismetMathLibrary.BreakVector` (`self.CurrentPosition`)))
  (bind _allcubelocations (`self.AllCubeLocations`))
  (bind (_stepxyz_x_2 _stepxyz_y_2 _stepxyz_z_2) (`KismetMathLibrary.BreakVector` (`self.StepXYZ`)))
  (bind _returnvalue (`StaticMesh.GetBoundingBox` (`self.Wall`)))
  (bind _returnvalue_2 (`StaticMesh.GetBoundingBox` (`self.Floor`)))
  (bind _returnvalue_3 (- (.x (`.Max` (break `Box` _returnvalue_2))) (.x (break `Box` _returnvalue_2))))
  (bind _returnvalue_4 (- (`KismetMathLibrary.Conv_IntToDouble` (`self.CubesOnOneSide`)) 3.0))
  ;[1 1 1] Lisa Sequence
  (`|ExecutionSequence`
    (:`then_0`
      ;[1 1 1] One Cube assembly measurements XYZ
      (set `self.StepXYZ` (`KismetMathLibrary.MakeVector` _returnvalue_3 _returnvalue_3 (+ (- (.z (`.Max` (break `Box` _returnvalue))) (.z (break `Box` _returnvalue))) (* (- (.z (`.Max` (break `Box` _returnvalue_2))) (.z (break `Box` _returnvalue_2))) 2.0)))))
    (:`then_1`
      ;[1 1 1] ArrayStepCubeSides -  Make Vector Array According to Amount of Cubes (27/64/125)
      (for _array_element (`self.Array122-212-221`)
        (`KismetArrayLibrary.Array_Add` _arraystepcubesides (+ _array_element (`KismetMathLibrary.MakeVector` _returnvalue_4 _returnvalue_4 _returnvalue_4))))
      ;[1 1 1] Get random
      (set `self.ArrayStepsFINAL` (`|GetArrayItem` _arraystepcubesides (- (`KismetMathLibrary.RandomInteger` (`KismetArrayLibrary.Array_Length` _arraystepcubesides)) 1))) ; StepCount ChosenOne (eg 1-0-1)
    )
    (:`then_2`
      ;[1 1 1] UnitVectorArrayNEW (3xVector3) -1 0 0 / 1 0 0 / 0 -1 0 / etc. SHUFFEL THE ORDER
      (`KismetArrayLibrary.Array_Add` _unitvectorarraynew (`KismetArrayLibrary.Array_Random` (`self.UnitVectorArray31`)))
      (`KismetArrayLibrary.Array_Add` _unitvectorarraynew (`KismetArrayLibrary.Array_Random` (`self.UnitVectorArray32`)))
      (`KismetArrayLibrary.Array_Add` _unitvectorarraynew (`KismetArrayLibrary.Array_Random` (`self.UnitVectorArray33`)))
      (`KismetArrayLibrary.Array_Shuffle` _unitvectorarraynew)
      ;[1 1 1] Making 1.CUBE
      (bind _vectorout (`self.CreateCube` (0.0 0.0 0.0)))
      (`KismetArrayLibrary.Array_Add` (`self.CorrectCubeLocations`) _vectorout)
      ;[1 1 1] 3 Unit Vectors Array - Making All Cubes
      (for _array_element_2 _unitvectorarraynew
        ;[1 1 1] Making a ROW of CUBES
        (for _ (range (+ (- (`self.CubesOnOneSide`) 2) 1))
          (bind _vectorout_2 (`self.CreateCube` (`KismetMathLibrary.MakeVector` (+ (* _stepxyz_x_2 (.x _array_element_2)) _currentposition_x) (+ (* _stepxyz_y_2 (.y _array_element_2)) _currentposition_y) (+ (* _stepxyz_z_2 (.z _array_element_2)) _currentposition_z))))
          (bind _output_get (set `self.CurrentPosition` _vectorout_2))
          (`KismetArrayLibrary.Array_Add` (`self.CorrectCubeLocations`) _output_get))))
    (:`then_4`
      ;[1 1 1] Make Death Cubes
      (for _array_element_3 (`self.CorrectCubeLocations`)
        (for _array_element_4 (`self.UnitVectorArray6`)
          (bind _returnvalue_5 (`KismetMathLibrary.MakeVector` (+ (* (.x _array_element_4) _stepxyz_x) (.x _array_element_3)) (+ (* (.y _array_element_4) _stepxyz_y) (.y _array_element_3)) (+ (* (.z _array_element_4) _stepxyz_z) (.z _array_element_3))))
          (if (not (or (`KismetArrayLibrary.Array_Contains` (`self.CorrectCubeLocations`) _returnvalue_5) (`KismetArrayLibrary.Array_Contains` (`self.DeathCubeLocations`) _returnvalue_5)))
            (`self.CreateCube` _returnvalue_5)
            (`KismetArrayLibrary.Array_AddUnique` (`self.DeathCubeLocations`) _returnvalue_5)))))
    (:`then_5`
      ;[1 1 1] All created Cubes to an Array in Player Controller
      (for _array_element_5 (`self.CorrectCubeLocations`)
        (`KismetArrayLibrary.Array_AddUnique` _allcubelocations _array_element_5))
      (for _array_element_6 (`self.DeathCubeLocations`)
        (`KismetArrayLibrary.Array_AddUnique` _allcubelocations _array_element_6)))
    (:`then_6`)))