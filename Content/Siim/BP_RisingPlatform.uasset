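; BP_RisingPlatform is a platform actor that moves up or down one room step on the player's choice.
; It adds a cube mesh and tagged box component at every RoomManager cube location, rebuilding on the coordinates-generated event.
; Player overlap events drive the up/down menu and input locking.
; Menu choices play timelines that lerp the whole actor vertically by StepXYZ.Z, with a DoOnce gate reset on end overlap.
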(event `self.ReceiveBeginPlay`
  (`KismetSystemLibrary.Delay` 0.2)
  (bind _asgame_instance_siim (cast `/Game/Siim/GameInstanceSiim` (`GameplayStatics.GetGameInstance`)))
  (bind _output_get (set `self.RoomManager` (`/Game/Siim/GameInstanceSiim.RoomManager` _asgame_instance_siim)))
  (add `/Game/Siim/BP_RoomManager.CoordinatesGenerated` _output_get (delegate `Create All Platforms`))
  (`self.Create All Platforms`)
  (bind _asplayer_controller_siim (cast `/Game/Siim/PlayerControllerSiim` (`GameplayStatics.GetPlayerController` 0)))
  (add `/Game/Siim/UI/UI_Up-Down.UpOrDown` (`/Game/Siim/UI/UI_Main.UI_Up-Down` (`/Game/Siim/PlayerControllerSiim.UI_Main` _asplayer_controller_siim)) (delegate `GoesUpOrDown`))
  (bind _asbp_third_person_character_siim (cast `/Game/Siim/BP_ThirdPersonCharacter_Siim` (`GameplayStatics.GetPlayerCharacter` 0)))
  (bind _output_get_2 (set `self.PlayerCharacter` _asbp_third_person_character_siim))
  (add `/Game/Siim/BP_ThirdPersonCharacter_Siim.PlayerBeginOverlapPlatform` _output_get_2 (`|CreateDelegate` :!event `ShowUpDownUI`))
  (add `/Game/Siim/BP_ThirdPersonCharacter_Siim.PlayerEndOverlapPlatform` _output_get_2 (`|CreateDelegate` :!event `EndOverlap`)))

(event `Create All Platforms`
  ;[1 1 1] Create Platforms
  (bind _asgame_instance_siim (cast `/Game/Siim/GameInstanceSiim` (`GameplayStatics.GetGameInstance`)))
  (for _array_element (`/Game/Siim/BP_RoomManager.AllCubeLocations` (`/Game/Siim/GameInstanceSiim.RoomManager` _asgame_instance_siim))
    (bind _returnvalue (`AddComponent|NODE_AddStaticMeshComponent-9` :`RelativeTransform` (`KismetMathLibrary.MakeTransform` _array_element)))
    (`StaticMeshComponent.SetStaticMesh` _returnvalue "/Game/Siim/SM/Cube_parts_Mesh3.Cube_parts_Mesh3")
    (bind _returnvalue_2 (`AddComponent|NODE_AddBoxComponent-2` :`RelativeTransform` (`KismetMathLibrary.MakeTransform` _array_element (struct) (0.05 0.05 3.0))))
    (set `ActorComponent.ComponentTags` (`self.TagArray`) _returnvalue_2)))

(event `GoesUpOrDown`
  (params (IsUp :type Boolean))
  (bind _currentlocation (`self.CurrentLocation`))
  (bind _x (.x _currentlocation))
  (bind _y (.y _currentlocation))
  (bind _z (.z _currentlocation))
  ;[1 1 1] UP-DOWN movement
  (bind _asgame_instance_siim (cast `/Game/Siim/GameInstanceSiim` (`GameplayStatics.GetGameInstance`)))
  (set `self.CurrentLocation` (`self.K2_GetActorLocation`))
  (`/Engine/EditorBlueprintResources/StandardMacros.DoOnce` false :!label _label
    (:`Completed`
      (if IsUp
        (bind (_direction _newtrack_0) (`Timeline|Timeline_0` :!via `PlayFromStart`)
          (:`Update`
            (bind (_stepxyz_x _stepxyz_y _stepxyz_z) (`KismetMathLibrary.BreakVector` (`/Game/Siim/BP_RoomManager.StepXYZ` (`/Game/Siim/GameInstanceSiim.RoomManager` _asgame_instance_siim))))
            (bind _returnvalue (`KismetMathLibrary.VLerp` _currentlocation (`KismetMathLibrary.MakeVector` _x _y (+ _z _stepxyz_z)) _newtrack_0))
            (`self.K2_SetActorLocation` _returnvalue true))
          (:`Finished`
            (set `self.CurrentLocation` _returnvalue)))
        (else
          (bind (_direction_2 _newtrack_0_2) (`Timeline|Timeline_1` :!via `PlayFromStart`)
            (:`Update`
              (bind _returnvalue_2 (`KismetMathLibrary.VLerp` _currentlocation (`KismetMathLibrary.MakeVector` _x _y (- _z _stepxyz_z)) _newtrack_0_2))
              (`self.K2_SetActorLocation` _returnvalue_2 true))
            (:`Finished`
              (set `self.CurrentLocation` _returnvalue_2))))))))

(event `EndOverlap`
  ;[1 1 1] UP-DOWN movement
  (`/Game/Siim/FunctionLibraryGeoMob.EnableInputAndMovement`)
  (goto _label :!via `Reset`))

(event `ShowUpDownUI`
  ;[1 1 1] Open Up-Down menu, disable outputs etc
  (bind _asplayer_controller_siim (cast `/Game/Siim/PlayerControllerSiim` (`GameplayStatics.GetPlayerController` 0)))
  (`Widget.SetVisibility` (`/Game/Siim/UI/UI_Main.UI_Up-Down` (`/Game/Siim/PlayerControllerSiim.UI_Main` _asplayer_controller_siim)) "Visible")
  (`/Game/Siim/FunctionLibraryGeoMob.DisableInputAndMovement`))

(fn `UserConstructionScript`)